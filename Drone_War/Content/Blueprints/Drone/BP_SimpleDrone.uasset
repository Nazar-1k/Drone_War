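; BP_SimpleDrone is a drone Blueprint that animates four spinning propellers and contains no flight or movement logic.
; BeginPlay resets a yaw accumulator, and each Tick adds a fixed step and applies it as relative rotation to all four propeller components.
; The step ignores delta time, so spin speed depends on frame rate, and all propellers turn in the same direction.
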(event `self.ReceiveBeginPlay`
  (set `self.New Rotation Z (Yaw)` 0.0))

(event `self.ReceiveTick`
  (params (DeltaSeconds :type "Float (single-precision)"))
  (bind _output_get (set `self.New Rotation Z (Yaw)` (+ 50.0 (`self.New Rotation Z (Yaw)`))))
  (`SceneComponent.K2_SetRelativeRotation` (`self.FrontLeftPropeler`) (`KismetMathLibrary.MakeRotator` 0.0 0.0 _output_get) false false)
  (`SceneComponent.K2_SetRelativeRotation` (`self.FrontRightPropeler`) (`KismetMathLibrary.MakeRotator` 0.0 0.0 _output_get) false false)
  (`SceneComponent.K2_SetRelativeRotation` (`self.BackRightPropeler`) (`KismetMathLibrary.MakeRotator` 0.0 0.0 _output_get) false false)
  (`SceneComponent.K2_SetRelativeRotation` (`self.BackLeftPropeler`) (`KismetMathLibrary.MakeRotator` 0.0 0.0 _output_get) false false))

(fn `UserConstructionScript`)